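; CameraActor is a camera rig that turns toward a target in the level and zooms according to its distance from it.
; BeginPlay caches a TargetActor found in the level, and each Tick sets the SpringArm's yaw to face it while preserving pitch and roll.
; Within LengthToZoom, the arm length blends linearly from MaxCameraZoom toward a fixed length as the target gets closer.
; The music variables are unused.
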(event EventBeginPlay
  (bind _returnvalue (Actor|GetActorOfClass "/Game/EndlessContent/Blueprints/TargetActor.TargetActor_C"))
  (Variables|Default|SetrotateTarget _returnvalue))

(event Collision|EventActorBeginOverlap
  (params (OtherActor :type Actor%20Object%20Reference)))

(event EventTick
  (params (DeltaSeconds :type Float%20%28single-precision%29))
  (bind _returnvalue (Transformation|GetActorLocation))
  (bind _rotatetarget (Variables|Default|GetrotateTarget))
  (bind _lengthtozoom (Variables|Default|GetlengthToZoom))
  (bind _springarm (Variables|Default|GetSpringArm))
  (bind _returnvalue_2 (Transformation|GetActorLocation _rotatetarget))
  (bind _returnvalue_3 (- _returnvalue_2 _returnvalue))
  (bind _returnvalue_4 (Math|Vector|VectorLength _returnvalue_3))
  ;[1 1 1] LookAtTarget
  (bind _output_get (Variables|Default|SetoldRot (Transformation|GetWorldRotation _springarm)))
  (Transformation|SetWorldRotation _springarm (Math|Rotator|MakeRotator (.roll _output_get) (.pitch _output_get) (.yaw (Math|Rotator|FindLookatRotation _returnvalue _returnvalue_2))) false false)
  (if (< _returnvalue_4 _lengthtozoom)
    (Variables|/Script/Engine.SpringArmComponent|SetTargetArmLength _springarm (Math|Float|Lerp (Variables|Default|GetmaxCameraZoom) 1.2e+03 (- 1.0 (/ _returnvalue_4 _lengthtozoom))))))

(fn ConstructionScript)