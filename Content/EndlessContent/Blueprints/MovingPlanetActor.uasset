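; MovingPlanetActor is an actor Blueprint that handles the movement and attack audio for a moving planet.
; On BeginPlay it assigns its movement and attack sound waves to two audio components, then starts the movement sound.
; Overlap with a PlayerPawn activates the attack sound, and leaving the overlap deactivates it.
; The graph itself contains no movement or damage logic.
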(event EventBeginPlay
  (|CallParentFunction)
  (bind _assound_wave (Utilities|Casting|CastToSoundWave (Variables|Default|GetMovementSound_1)))
  (Audio|Components|Audio|SetSound (Variables|Default|GetMovementSound_Cue) _assound_wave)
  (bind _assound_wave_2 (Utilities|Casting|CastToSoundWave (Variables|Default|GetAttackSound_1)))
  (Audio|Components|Audio|SetSound (Variables|Default|GetAttack_Cue) _assound_wave_2)
  (Components|Activation|Activate (Variables|Default|GetMovementSound_Cue) false))

(event Collision|EventActorEndOverlap
  (params (OtherActor :type Actor%20Object%20Reference))
  (if (== (Utilities|GetClass OtherActor) "/Game/EndlessContent/Blueprints/PlayerPawn.PlayerPawn_C")
    (Components|Activation|Deactivate (Variables|Default|GetAttack_Cue))))

(event Collision|EventActorBeginOverlap
  (params (OtherActor :type Actor%20Object%20Reference))
  (if (== (Utilities|GetClass OtherActor) "/Game/EndlessContent/Blueprints/PlayerPawn.PlayerPawn_C")
    (Components|Activation|Activate (Variables|Default|GetAttack_Cue) false)))

(fn ConstructionScript
  (|CallParentFunction))