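; FlyweightGenerator spawns layered grids of Flyweight actors when play begins.
; It loops over depth levels, rows and columns, with per-level arrays setting grid size, spacing, Z height, position variance and XY scale.
; Each spawn gets random XY and depth jitter plus a random yaw, breaking up the regularity of the grid.
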(event EventBeginPlay
  (bind _currentdepth (Variables|Default|GetcurrentDepth))
  (bind _maxvarianceposition (Variables|Default|GetmaxVariancePosition))
  (bind _currentdepth_2 (Variables|Default|GetcurrentDepth))
  (bind _scale (Variables|Default|Getscale))
  (bind _maxvariancedepth (Variables|Default|GetmaxVarianceDepth))
  (bind _positionoffset (Variables|Default|GetpositionOffset))
  (bind _maxvarianceposition_2 (Variables|Default|GetmaxVariancePosition))
  (bind _output (Utilities|Array|Get(acopy) _maxvarianceposition_2 _currentdepth_2))
  (bind _output_2 (Utilities|Array|Get(acopy) _maxvarianceposition _currentdepth_2))
  (bind _output_3 (Utilities|Array|Get(acopy) _positionoffset _currentdepth_2))
  (bind _output_4 (Utilities|Array|Get(acopy) _scale _currentdepth))
  ;[1 1 1] generating flyweight loop
  (Variables|Default|SetcurrentRow 0)
  (while (< _currentdepth_2 (Variables|Default|GetzDepthLevels))
    (Variables|Default|SetcurrentRow 0)
    (while (< (Variables|Default|GetcurrentRow) (Utilities|Array|Get(acopy) (Variables|Default|GetrowAmmount) _currentdepth_2))
      (Variables|Default|SetcurrentColumn 0)
      (while (< (Variables|Default|GetcurrentColumn) (Utilities|Array|Get(acopy) (Variables|Default|GetcolumnAmmount) _currentdepth_2))
        (Game|SpawnActorfromClass "/Game/EndlessContent/Blueprints/FXBlueprint/Flyweight.Flyweight_C" (Math|Transform|MakeTransform (Math|Vector|MakeVector (+ (Math|Random|RandomFloatinRange (* _output -1.0) _output) (Math|Conversions|ToFloat(Integer) (* (Variables|Default|GetcurrentColumn) _output_3))) (+ (Math|Random|RandomFloatinRange (* _output_2 -1.0) _output_2) (Math|Conversions|ToFloat(Integer) (* (Variables|Default|GetcurrentRow) _output_3))) (+ (Math|Conversions|ToFloat(Integer) (Utilities|Array|Get(acopy) (Variables|Default|GetzPosition) _currentdepth)) (Math|Random|RandomFloatinRange (* _maxvariancedepth -1.0) _maxvariancedepth))) (Math|Rotator|MakeRotator 0.0 0.0 (Math|Random|RandomFloatinRange 0.0 3.6e+02)) (Math|Vector|MakeVector _output_4 _output_4 1.0)) "Undefined" 0 0)
        (Math|Integer|IncrementInt (Variables|Default|GetcurrentColumn)))
      (Math|Integer|IncrementInt (Variables|Default|GetcurrentRow)))
    (Math|Integer|IncrementInt (Variables|Default|GetcurrentDepth))))

(event Collision|EventActorBeginOverlap
  (params (OtherActor :type Actor%20Object%20Reference)))

(event EventTick
  (params (DeltaSeconds :type Float%20%28single-precision%29)))

(fn ConstructionScript)