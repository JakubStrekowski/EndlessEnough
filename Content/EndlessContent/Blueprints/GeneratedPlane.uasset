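; GeneratedPlane is a plane actor that randomizes its material and footprint when play begins.
; It picks a material from MaterialList by random index, though the last entry is never chosen.
; Its world Z, matched as a string against three fixed heights, selects the random range for independent X and Y scales, with lower planes growing larger.
; Any other height leaves the scale unchanged.
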(event EventBeginPlay
  (bind _returnvalue (Math|Random|RandomFloatinRange 25.0 4e+01))
  (bind _returnvalue_2 (Math|Random|RandomFloatinRange 0.5 3.0))
  (bind _returnvalue_3 (Math|Random|RandomFloatinRange 4.0 1e+01))
  (bind _materiallist (Variables|Default|GetmaterialList))
  (bind _staticmeshcomponent (Variables|Debug|GetStaticMeshComponent))
  (Rendering|Material|SetMaterial _staticmeshcomponent 0 (Utilities|Array|Get(acopy) _materiallist (Math|Random|RandomInteger (Utilities|Array|LastIndex _materiallist))))
  (switch string (Utilities|String|ToString(Float) (.z (Transformation|GetActorLocation)))
    (:-10.0
      (Variables|Default|SetscalePlaneX _returnvalue_2)
      (Variables|Default|SetscalePlaneY _returnvalue_2))
    (:-20.0
      (Variables|Default|SetscalePlaneX _returnvalue_3)
      (Variables|Default|SetscalePlaneY _returnvalue_3))
    (:-30.0
      (Variables|Default|SetscalePlaneX _returnvalue)
      (Variables|Default|SetscalePlaneY _returnvalue)))
  (Transformation|SetWorldScale3D _staticmeshcomponent (Math|Vector|MakeVector (Variables|Default|GetscalePlaneX) (Variables|Default|GetscalePlaneY) 1.0)))

(event EventTick
  (params (DeltaSeconds :type Float%20%28single-precision%29)))

(fn ConstructionScript)