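; Level light Blueprint in EndlessContent that sets directional light intensity from the player pawn's distance to its target.
; On BeginPlay, after a short delay, it finds the PlayerPawn and stores its DistanceToTarget as the starting distance, printing it for debug.
; Each Tick it linearly maps the current-to-starting distance ratio to intensity, so the light brightens as the pawn nears the target.
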(event EventBeginPlay
  ;[1 1 1] okersla intensywnosc oswietlenia poziomu na podstawie odleglosci pawActor od targetActor
  (Utilities|FlowControl|Delay 0.2)
  (bind _returnvalue (Actor|GetActorOfClass "/Game/EndlessContent/Blueprints/PlayerPawn.PlayerPawn_C"))
  (bind _output_get (Variables|Default|SetplayerActor _returnvalue))
  (bind _asplayer_pawn (Utilities|Casting|CastToPlayerPawn _output_get))
  (Variables|Default|SetstartingDistance (Variables|/Game/EndlessContent/Blueprints/PlayerPawn.PlayerPawn_C|GetDistanceToTarget _asplayer_pawn))
  (Development|PrintString (Utilities|String|ToString(Float) (Variables|/Game/EndlessContent/Blueprints/PlayerPawn.PlayerPawn_C|GetDistanceToTarget _asplayer_pawn))))

(event EventTick
  (params (DeltaSeconds :type Float%20%28single-precision%29))
  ;[1 1 1] okersla intensywnosc oswietlenia poziomu na podstawie odleglosci pawActor od targetActor
  (bind _asplayer_pawn (Utilities|Casting|CastToPlayerPawn (Variables|Default|GetplayerActor)))
  (bind _output_get (Variables|Default|SetcurrentDistance (Variables|/Game/EndlessContent/Blueprints/PlayerPawn.PlayerPawn_C|GetDistanceToTarget _asplayer_pawn)))
  (Rendering|Components|Light|SetIntensity (Variables|DayNightCycle|GetDirectionalLightComponent) (+ (* (- 1.0 (/ _output_get (Variables|Default|GetstartingDistance))) 5.0) 2.0)))

(fn ConstructionScript)